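; Physics-driven boid particle that flocks once activated, shrinks every tick, and destroys itself when tiny or on hitting anything but another boid.
; Each active tick it scans all BoidBP actors, applying cohesion, alignment and separation forces from neighbours in range.
; It also adds a constant +Y force and a push from the "Fan"-tagged actor while Overlapping, then clamps velocity to a fixed Speed.
; The face-velocity rotation is unwired.
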(event EventBeginPlay
  (bind _outactors (Actor|GetAllActorswithTag "Fan"))
  (for _array_element _outactors
    (Variables|Default|SetFan _array_element)))

(event EventTick
  (params (DeltaSeconds :type Float%20%28single-precision%29))
  (bind _staticmesh (Variables|Components|GetStaticMesh))
  (bind _staticmesh_2 (Variables|Components|GetStaticMesh))
  (bind _returnvalue (Transformation|GetWorldLocation _staticmesh_2))
  (CallFunction|Shrink)
  (if (Variables|Default|Getactive)
    (Utilities|FlowControl|Sequence
      (:then_0
        (if (Variables|Default|Getoverlapping)
          (Physics|AddForce (Variables|Components|GetStaticMesh) (* (Transformation|GetActorForwardVector (Variables|Default|GetFan)) 2e+01) "None" false)))
      (:then_1
        (Physics|AddForce (Variables|Components|GetStaticMesh) "0,1.000000, 0" "None" false))
      (:then_2
        (bind _outactors (Actor|GetAllActorsOfClass "BoidBP_C"))
        (Variables|Default|SetAvgPos "0, 0, 0")
        (Variables|Default|SetCounter 0)
        (Variables|Default|SetAvgDis "0, 0, 0")
        (Variables|Default|SetSeppCounter 0)
        (Variables|Default|SetAvgDir "0, 0, 0")
        (for _array_element _outactors
          (if (not (Math|Vector|Equal(Vector) (Transformation|GetWorldLocation (Variables|BoidBP_C|GetStaticMesh _array_element)) _returnvalue 0.1))
            (Math|Float|CompareFloat (Math|Vector|VectorLength (- (Transformation|GetWorldLocation (Variables|BoidBP_C|GetStaticMesh _array_element)) _returnvalue)) (Variables|Default|GetViewRange)
              (:<
                (Utilities|FlowControl|Sequence
                  (:then_0
                    (bind _returnvalue_2 (Physics|GetPhysicsLinearVelocity (Variables|BoidBP_C|GetStaticMesh _array_element) "None"))
                    (Variables|Default|SetAvgDir (+ (Variables|Default|GetAvgDir) _returnvalue_2)))
                  (:then_1
                    (Variables|Default|SetAvgPos (+ (Variables|Default|GetAvgPos) (- (Transformation|GetWorldLocation (Variables|BoidBP_C|GetStaticMesh _array_element)) _returnvalue)))
                    (Math|Integer|IncrementInt (Variables|Default|GetCounter)))
                  (:then_2
                    (Math|Float|CompareFloat (Math|Vector|VectorLength (- (Transformation|GetWorldLocation (Variables|BoidBP_C|GetStaticMesh _array_element)) _returnvalue)) (Variables|Default|GetSeparateRange)
                      (:<
                        (Variables|Default|SetAvgDis (+ (Variables|Default|GetAvgDis) (* (- (Transformation|GetWorldLocation (Variables|BoidBP_C|GetStaticMesh _array_element)) _returnvalue) (/ -1.0 (Math|Vector|VectorLength (- (Transformation|GetWorldLocation (Variables|BoidBP_C|GetStaticMesh _array_element)) _returnvalue))))))
                        (Math|Integer|IncrementInt (Variables|Default|GetSeppCounter))))))))))
        (Math|Integer|CompareInt (Variables|Default|GetCounter)
          (:>
            (Physics|AddForce (Variables|Components|GetStaticMesh) (* (/ (Variables|Default|GetAvgPos) (Math|Conversions|ToFloat(Integer) (Variables|Default|GetCounter))) (Variables|Default|GetCoheseRate)) "None" false)
            (Physics|AddForce (Variables|Components|GetStaticMesh) (* (Math|Vector|Normalize (Variables|Default|GetAvgDir)) (Variables|Default|GetAlignRate)) "None" false)
            (Math|Integer|CompareInt (Variables|Default|GetSeppCounter)
              (:>
                (Physics|AddForce (Variables|Components|GetStaticMesh) (* (/ (Variables|Default|GetAvgDis) (Math|Conversions|ToFloat(Integer) (Variables|Default|GetSeppCounter))) (Variables|Default|GetSeparateRate)) "None" false))))))
      (:then_3
        (bind _returnvalue_3 (Physics|GetPhysicsLinearVelocity (Variables|Components|GetStaticMesh) "None"))
        (bind _returnvalue_4 (Physics|GetPhysicsLinearVelocity _staticmesh "None"))
        (Class|PrimitiveComponent|SetAllPhysicsLinearVelocity _staticmesh (* (Math|Vector|Normalize _returnvalue_4) (Variables|Default|GetSpeed)) false)))))

(event Collision|EventHit
  (params (MyComp :type Primitive%20Component%20Object%20Reference) (Other :type Actor%20Object%20Reference) (OtherComp :type Primitive%20Component%20Object%20Reference) (bSelfMoved :type Boolean) (HitLocation :type Vector :default "0, 0, 0") (HitNormal :type Vector :default "0, 0, 0") (NormalImpulse :type Vector :default "0, 0, 0") (Hit :type Hit%20Result%20Structure%20%28by%20ref%29))
  (Utilities|Casting|CastToBoidBP Other
    (:CastFailed
      (Utilities|FlowControl|DoOnce false
        (:Completed
          (Actor|DestroyActor))))))

(fn ConstructionScript)

(fn SetActive
  (Variables|Default|Setactive true)
  (Rendering|Material|SetMaterial (Variables|Components|GetStaticMesh) 0 "/Game/MainContent/Materials/Emissive/EParticleActive.EParticleActive"))

(fn SetSpeed
  (params (Speed :type Float%20%28single-precision%29))
  (Variables|Default|SetSpeed Speed))

(fn Shrink
  (bind _staticmesh (Variables|Components|GetStaticMesh))
  (bind _returnvalue (Transformation|GetRelativeTransform _staticmesh))
  (bind _returnvalue_2 (* (.scale _returnvalue) 0.999))
  (if (Math|Vector|Equal(Vector) _returnvalue_2 "0, 0, 0" 0.001)
    (Actor|DestroyActor)
    (else
      (Transformation|SetRelativeScale3D (Variables|Components|GetStaticMesh) _returnvalue_2))))