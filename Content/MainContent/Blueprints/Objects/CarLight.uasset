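; CarLight is a looping moving actor, by its name a car light, that drifts along the X axis.
; BeginPlay stores its start location, then places it at a random X offset behind that point with a random speed.
; Tick adds that speed to X every frame, without delta-time scaling, and jumps back to the same randomization once world X passes a hard-coded limit.
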(event EventBeginPlay
  (Variables|Default|SetStart (Transformation|GetActorLocation))
  (Transformation|SetActorLocation (Math|Vector|MakeVector (+ (Math|Random|RandomFloatinRange -1e+03 0.0) (.X (Math|Vector|BreakVector (Variables|Default|GetStart)))) (.Y (Math|Vector|BreakVector (Variables|Default|GetStart))) (.Z (Math|Vector|BreakVector (Variables|Default|GetStart)))) false false)
  (Variables|Default|Setspeed (Math|Random|RandomFloatinRange 1.0 4.0)))

(event Collision|EventActorBeginOverlap
  (params (OtherActor :type Actor%20Object%20Reference)))

(event EventTick
  (params (DeltaSeconds :type Float%20%28single-precision%29))
  (bind _start (Variables|Default|GetStart))
  (bind (_x _y _z) (Math|Vector|BreakVector _start))
  (Transformation|AddRelativeLocation (Variables|Default|GetDefaultSceneRoot) (Math|Vector|MakeVector (Variables|Default|Getspeed) 0.0 0.0) false false)
  (Math|Float|CompareFloat (.x (Transformation|GetActorLocation)) -3e+02
    (:>
      (Transformation|SetActorLocation (Math|Vector|MakeVector (+ (Math|Random|RandomFloatinRange -1e+03 0.0) _x) _y _z) false false)
      (Variables|Default|Setspeed (Math|Random|RandomFloatinRange 1.0 4.0)))))

(fn ConstructionScript)